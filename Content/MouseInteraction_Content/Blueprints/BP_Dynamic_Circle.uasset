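; Dynamic circle for a timing minigame, where a click stops it as it grows or shrinks toward and past the size of BP_Static_Circle.
; SetDynamicCircle copies the static circle's color, picks a random smaller or larger start size, then plays a timeline that lerps the scale.
; Stopping prints a rating from the size difference, timeline completion prints MISS, and both then update the static circle.
; MenuAI auto-stops the timeline after a random delay when not playing.
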(event OnClicked(DynamicCircleMesh)
  (params (TouchedComponent :type Primitive%20Component%20Object%20Reference) (ButtonPressed :type Key%20Structure :default "None"))
  (if (Variables|Default|GetbIsPlayingGame)
    (Utilities|ClickonCircles (Variables|Default|GetbCanInput)
      (:Out
        (Utilities|CompareSizeOfCircles
          (:Out
            (Utilities|FlowControl|Delay 0.75)
            (Default|UpdateStaticCircle (Variables|Default|GetStatic%20Circle%20Reference))
            (Utilities|FlowControl|Delay 0.5)
            (Variables|Default|SetbCanInput true)))))))

(event Custom|Set%20Dynamic%20Circle
  (CallFunction|SetDynamicCircleColor)
  (Utilities|SetSizeOfDynamicCircle
    (:Out
      (Components|Timeline|PlayfromStart (Variables|Default|GetScale%20Dynamic%20Circle)))))

(event Custom|Click%20Static%20Circle
  (if (Variables|Default|GetbIsPlayingGame)
    (Utilities|ClickonCircles (Variables|Default|GetbCanInput)
      (:Out
        (Utilities|CompareSizeOfCircles
          (:Out
            (Utilities|FlowControl|Delay 0.75)
            (Default|UpdateStaticCircle (Variables|Default|GetStatic%20Circle%20Reference))
            (Utilities|FlowControl|Delay 0.5)
            (Variables|Default|SetbCanInput true)))))))

(event Custom|Menu%20AI
  (if (not (Variables|Default|GetbIsPlayingGame))
    (Components|Timeline|SetPlayRate (Variables|Default|GetScale%20Dynamic%20Circle) 1.0)
    (Utilities|FlowControl|Delay (Math|Random|RandomFloatinRange 0.9 1.4))
    (Audio|Components|Audio|Stop (Variables|Default|GetScale%20Dynamic%20Circle))
    (Utilities|CompareSizeOfCircles
      (:Out
        (Utilities|FlowControl|Delay 0.5)
        (Components|Timeline|SetPlaybackPosition (Variables|Default|GetScale%20Dynamic%20Circle) 0.0 false true)
        (Default|UpdateStaticCircle (Variables|Default|GetStatic%20Circle%20Reference))))))

(event EventBeginPlay)

(event Collision|EventActorBeginOverlap
  (params (OtherActor :type Actor%20Object%20Reference)))

(event EventTick
  (params (DeltaSeconds :type Float%20%28single-precision%29)))

(fn ConstructionScript
  (bind _outactors (Actor|GetAllActorsOfClass "/Game/MouseInteraction_Content/Blueprints/BP_Static_Circle.BP_Static_Circle_C"))
  (bind _asbp_static_circle (Utilities|Casting|CastToBP_Static_Circle (Utilities|Array|Get(acopy) _outactors)))
  (Variables|Default|SetStatic%20Circle%20Reference _asbp_static_circle)
  (bind _returnvalue (Rendering|Material|CreateDynamicMaterialInstance (Variables|Default|GetDynamic%20Circle%20Mesh) 0 0 "None" :!class /Script/Engine.PrimitiveComponent))
  (Variables|Default|SetDynamic%20Circle%20MI _returnvalue))

(fn SetDynamicCircleColor
  (bind _returnvalue (Rendering|Material|GetVectorParameterValue (Variables|/Game/MouseInteraction_Content/Blueprints/BP_Static_Circle.BP_Static_Circle_C|GetStatic%20Circle%20MI (Variables|Default|GetStatic%20Circle%20Reference)) "Static Circle Color" :!class /Script/Engine.MaterialInstanceDynamic))
  (Variables|Default|SetStatic%20Circle%20Color _returnvalue)
  (Rendering|Material|SetVectorParameterValue (Variables|Default|GetDynamic%20Circle%20MI) "Dynamic Circle Color" (Variables|Default|GetStatic%20Circle%20Color) :!class /Script/Engine.MaterialInstanceDynamic))