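; BP_TimeTrials_Button is a clickable 3D Time Trials button that gives animated mouse feedback.
; The construction script creates a dynamic material instance, which a timeline uses to brighten button and text intensity on hover and reverse on cursor exit.
; Clicking plays a second timeline that scales the mesh, with no other action in this Blueprint.
; Click and hover-in respond only while the mesh is visible.
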(event OnClicked(TimeTrialsButtonMesh)
  (params (TouchedComponent :type Primitive%20Component%20Object%20Reference) (ButtonPressed :type Key%20Structure :default "None"))
  (if (Rendering|IsVisible (Variables|Default|GetTime%20Trials%20Button%20Mesh))
    (bind _button_scale (Timeline|Time%20Trials%20Time%20Scale PlayFromStart)
      (:Update
        (Transformation|SetRelativeScale3D (Variables|Default|GetTime%20Trials%20Button%20Mesh) (Math|Vector|Lerp(Vector) "1.000000,1.000000,1.000000" "1.200000,1.200000,1.200000" _button_scale))))))

(event OnBeginCursorOver(TimeTrialsButtonMesh)
  (params (TouchedComponent :type Primitive%20Component%20Object%20Reference))
  (if (Rendering|IsVisible (Variables|Default|GetTime%20Trials%20Button%20Mesh))
    (bind _emissive_flash (Timeline|Time%20Trials%20Button%20Emissive%20Flash PlayFromStart)
      (:Update
        (Rendering|Material|SetScalarParameterValue (Variables|Default|GetTime%20Trials%20Button%20MI) "Time Trials Button Text Intensity" (Math|Float|Lerp 0.1 0.3 _emissive_flash) :!class /Script/Engine.MaterialInstanceDynamic)
        (Rendering|Material|SetScalarParameterValue (Variables|Default|GetTime%20Trials%20Button%20MI) "Time Trials Button Intensity" (Math|Float|Lerp 0.1 0.6 _emissive_flash) :!class /Script/Engine.MaterialInstanceDynamic)))))

(event OnEndCursorOver(TimeTrialsButtonMesh)
  (params (TouchedComponent :type Primitive%20Component%20Object%20Reference))
  (bind _emissive_flash (Timeline|Time%20Trials%20Button%20Emissive%20Flash ReverseFromEnd)
    (:Update
      (Rendering|Material|SetScalarParameterValue (Variables|Default|GetTime%20Trials%20Button%20MI) "Time Trials Button Text Intensity" (Math|Float|Lerp 0.1 0.3 _emissive_flash) :!class /Script/Engine.MaterialInstanceDynamic)
      (Rendering|Material|SetScalarParameterValue (Variables|Default|GetTime%20Trials%20Button%20MI) "Time Trials Button Intensity" (Math|Float|Lerp 0.1 0.6 _emissive_flash) :!class /Script/Engine.MaterialInstanceDynamic))))

(event EventBeginPlay)

(event Collision|EventActorBeginOverlap
  (params (OtherActor :type Actor%20Object%20Reference)))

(event EventTick
  (params (DeltaSeconds :type Float%20%28single-precision%29)))

(fn ConstructionScript
  (bind _returnvalue (Rendering|Material|CreateDynamicMaterialInstance (Variables|Default|GetTime%20Trials%20Button%20Mesh) 0 0 "None" :!class /Script/Engine.PrimitiveComponent))
  (Variables|Default|SetTime%20Trials%20Button%20MI _returnvalue))