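; Clickable target circle for a mouse-interaction game, paired with the BP_Dynamic_Circle found in the construction script.
; On BeginPlay or UpdateStaticCircle it moves both circles to a random spot on a fixed Y plane, then randomizes its scale, dominant-RGB color and glow intensity via a dynamic material instance before calling SetDynamicCircle.
; Clicks are forwarded to the dynamic circle during play; otherwise each refresh triggers its MenuAI.
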(event OnClicked(StaticCircleMesh)
  (params (TouchedComponent :type Primitive%20Component%20Object%20Reference) (ButtonPressed :type Key%20Structure :default "None"))
  (if (Variables|/Game/MouseInteraction_Content/Blueprints/BP_Dynamic_Circle.BP_Dynamic_Circle_C|GetbIsPlayingGame (Variables|Default|GetDynamic%20Circle%20Reference))
    (Default|ClickStaticCircle (Variables|Default|GetDynamic%20Circle%20Reference))))

(event Custom|Update%20Static%20Circle
  (if (Variables|/Game/MouseInteraction_Content/Blueprints/BP_Dynamic_Circle.BP_Dynamic_Circle_C|GetbIsPlayingGame (Variables|Default|GetDynamic%20Circle%20Reference))
    _
    (else
      (Development|PrintString "Menu AI Playing")
      (Default|MenuAI (Variables|Default|GetDynamic%20Circle%20Reference))))
  (Utilities|ChangeCirclesLocation
    (:Out
      (Utilities|GenerateRandomColor (Math|Random|RandomIntegerinRange 0 2)
        (:Out
          (Utilities|SetRandomCircleScale
            (:Out
              (Rendering|Material|SetScalarParameterValue (Variables|Default|GetStatic%20Circle%20MI) "Static Circle Intensity" (Math|Random|RandomFloatinRange 4.0 8.0) :!class /Script/Engine.MaterialInstanceDynamic)
              (Default|SetDynamicCircle (Variables|Default|GetDynamic%20Circle%20Reference)))))))))

(event Collision|EventActorBeginOverlap
  (params (OtherActor :type Actor%20Object%20Reference)))

(event EventTick
  (params (DeltaSeconds :type Float%20%28single-precision%29)))

(event EventBeginPlay
  (if (Variables|/Game/MouseInteraction_Content/Blueprints/BP_Dynamic_Circle.BP_Dynamic_Circle_C|GetbIsPlayingGame (Variables|Default|GetDynamic%20Circle%20Reference))
    _
    (else
      (Development|PrintString "Menu AI Playing")
      (Default|MenuAI (Variables|Default|GetDynamic%20Circle%20Reference))))
  (Utilities|ChangeCirclesLocation
    (:Out
      (Utilities|GenerateRandomColor (Math|Random|RandomIntegerinRange 0 2)
        (:Out
          (Utilities|SetRandomCircleScale
            (:Out
              (Rendering|Material|SetScalarParameterValue (Variables|Default|GetStatic%20Circle%20MI) "Static Circle Intensity" (Math|Random|RandomFloatinRange 4.0 8.0) :!class /Script/Engine.MaterialInstanceDynamic)
              (Default|SetDynamicCircle (Variables|Default|GetDynamic%20Circle%20Reference)))))))))

(fn ConstructionScript
  (bind _returnvalue (Rendering|Material|CreateDynamicMaterialInstance (Variables|Default|GetStatic%20Circle%20Mesh) 0 0 "None" :!class /Script/Engine.PrimitiveComponent))
  (Variables|Default|SetStatic%20Circle%20MI _returnvalue)
  (Variables|Default|SetDefault%20Static%20Circle%20Scale (Variables|/Script/Engine.SceneComponent|GetRelativeScale3D (Variables|Default|GetStatic%20Circle%20Mesh)))
  (bind _outactors (Actor|GetAllActorsOfClass "/Game/MouseInteraction_Content/Blueprints/BP_Dynamic_Circle.BP_Dynamic_Circle_C"))
  (bind _asbp_dynamic_circle (Utilities|Casting|CastToBP_Dynamic_Circle (Utilities|Array|Get(acopy) _outactors)))
  (Variables|Default|SetDynamic%20Circle%20Reference _asbp_dynamic_circle))